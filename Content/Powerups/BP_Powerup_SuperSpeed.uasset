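; Speed powerup that temporarily doubles the walk speed of the player it activates for.
; OnActivated stores that player and doubles the MaxWalkSpeed on its CharacterMovementComponent.
; OnExpired halves the current value if the stored player is still valid, then calls the parent's expiry logic.
; The change is relative, so no original speed is cached.
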(event EventOnActivated
  (params (ActivateFor :type Actor%20Object%20Reference))
  (bind _returnvalue (Actor|GetComponentbyClass ActivateFor "/Script/Engine.CharacterMovementComponent"))
  (Variables|Default|SetActivatedForPlayer ActivateFor)
  (Variables|/Script/Engine.CharacterMovementComponent|SetMaxWalkSpeed _returnvalue (* (Variables|/Script/Engine.CharacterMovementComponent|GetMaxWalkSpeed _returnvalue) 2.0)))

(event EventOnExpired
  (bind _activatedforplayer (Variables|Default|GetActivatedForPlayer))
  (bind _returnvalue (Actor|GetComponentbyClass _activatedforplayer "/Script/Engine.CharacterMovementComponent"))
  (Utilities|IsValid _activatedforplayer
    (:Is%20Valid
      (Variables|/Script/Engine.CharacterMovementComponent|SetMaxWalkSpeed _returnvalue (/ (Variables|/Script/Engine.CharacterMovementComponent|GetMaxWalkSpeed _returnvalue) 2.0)))
    (:Is%20Not%20Valid
      _))
  (|CallParentFunction))

(fn ConstructionScript)